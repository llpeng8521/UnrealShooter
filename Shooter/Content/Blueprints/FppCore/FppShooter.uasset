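; First-person shooter character that moves, looks, fires and cycles between a rifle and a launcher.
; On BeginPlay it spawns both guns attached to the mesh's right-hand weapon socket, hidden except the active one.
; Fire input forwards start and end calls to the current gun.
; Switching stops firing, swaps visibility and plays an equip montage, while a timestamp check briefly blocks new shots and further switches.
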(event `self.ReceiveBeginPlay`
  (`self.CreateGun` "/Game/Blueprints/Rifle.Rifle_C")
  (`self.CreateGun` "/Game/Blueprints/Launcher.Launcher_C")
  (set `self.CurrentGunIndex` 0)
  (`self.SetActorHiddenInGame` (`self.GetCurrentGun`) false))

(event `InputAxis|MoveForward`
  (params (AxisValue :type "Float (single-precision)"))
  (`self.AddMovementInput` (`KismetMathLibrary.GetForwardVector` (`self.GetControlRotation`)) AxisValue))

(event `InputAxis|MoveRight`
  (params (AxisValue :type "Float (single-precision)"))
  (`self.AddMovementInput` (`KismetMathLibrary.GetRightVector` (`self.GetControlRotation`)) AxisValue))

(event `InputAxis|Turn`
  (params (AxisValue :type "Float (single-precision)"))
  (`self.AddControllerYawInput` AxisValue))

(event `InputAxis|Lookup`
  (params (AxisValue :type "Float (single-precision)"))
  (`self.AddControllerPitchInput` AxisValue))

(event `InputAction|Fire`
  (params (Key :type "Key Structure"))
  (:`Pressed`
    (`self.StartFire`))
  (:`Released`
    (`self.EndFire`)))

(event `InputAction|Equip`
  (params (Key :type "Key Structure"))
  (:`Pressed`
    (`self.SwitchWeapon`)))

(fn `CreateGun`
  (params (Gun :type "/Game/Blueprints/Gun Class Reference"))
  (bind _returnvalue (`|SpawnActorFromClass` Gun (`KismetMathLibrary.MakeTransform` (0.0 0.0 0.0)) "Undefined" "OverrideRootScale" null null))
  (`self.K2_AttachToComponent` _returnvalue (`self.Mesh`) "RightWeaponSocket" "SnapToTarget" "SnapToTarget" "SnapToTarget" true)
  (set `/Game/Blueprints/Gun.GunOwner` self _returnvalue)
  (`KismetArrayLibrary.Array_Add` (`self.Guns`) _returnvalue)
  (`self.SetActorHiddenInGame` _returnvalue true))

(fn `EndFire`
  (`/Game/Blueprints/Gun.EndFire` (`self.GetCurrentGun`)))

(fn `GetCurrentGun`
  (returns (Gun :type "/Game/Blueprints/Gun Object Reference"))
  (return (`|GetArrayItem` (`self.Guns`) (`self.CurrentGunIndex`))))

(fn `IsInEquip`
  (returns (Equipping :type Boolean))
  (return (< (- (`GameplayStatics.GetTimeSeconds`) (`self.EquipTime`)) 0.6)))

(fn `StartFire`
  (if (not (`self.IsInEquip`))
    (`/Game/Blueprints/Gun.StartFire` (`self.GetCurrentGun`))))

(fn `SwitchWeapon`
  (if (not (`self.IsInEquip`))
    (`self.EndFire`)
    (`self.SetActorHiddenInGame` (`self.GetCurrentGun`) true)
    (set `self.CurrentGunIndex` (mod (+ (`self.CurrentGunIndex`) 1) (`KismetArrayLibrary.Array_Length` (`self.Guns`))))
    (`self.SetActorHiddenInGame` (`self.GetCurrentGun`) false)
    (`self.PlayAnimMontage` "/Game/Blueprints/FppCore/FppEquip_Montage.FppEquip_Montage")
    (set `self.EquipTime` (`GameplayStatics.GetTimeSeconds`))))

(fn `UserConstructionScript`
  (`PrimitiveComponent.SetCollisionResponseToChannel` (`self.Mesh`) "ECC_Visibility" "ECR_Block"))