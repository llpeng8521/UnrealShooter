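; Rifle weapon Blueprint that gives its owner automatic hitscan fire against RobotShooter targets.
; StartFire plays the owner's first-person fire montage, attaches a muzzle flash and repeats ShootOnce on a looping timer until EndFire undoes all three.
; ShootOnce line-traces a short range from the owner's camera along control rotation, with debug drawing, and deals fixed damage to any RobotShooter hit.
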(event `self.StartFire`
  (`|ExecutionSequence`
    (:`then_0`
      (`Character.PlayAnimMontage` (`self.GunOwner`) "/Game/Blueprints/FppCore/FppRifleFire_Montage.FppRifleFire_Montage" 1.0 "None")
      (bind _returnvalue (`GameplayStatics.SpawnEmitterAttached` "/Game/Assets/Effects/ParticleSystems/Weapons/AssaultRifle/Muzzle/P_AssaultRifle_MF.P_AssaultRifle_MF" (`self.Muzzle`)))
      (set `self.FireEffects` _returnvalue))
    (:`then_1`
      (`self.ShootOnce`)
      (`KismetSystemLibrary.K2_SetTimer` null "ShootOnce" 0.2 true))
    (:`then_2`
      (set `self.IsInFire` true))))

(event `self.EndFire`
  (if (`self.IsInFire`)
    (`|ExecutionSequence`
      (:`then_0`
        (`Character.StopAnimMontage` (`self.GunOwner`) "/Game/Blueprints/FppCore/FppRifleFire_Montage.FppRifleFire_Montage")
        (`ActorComponent.K2_DestroyComponent` (`self.FireEffects`)))
      (:`then_1`
        (`KismetSystemLibrary.K2_ClearTimer` null "ShootOnce"))
      (:`then_2`
        (set `self.IsInFire` false)))))

(event `self.ShootOnce`
  (bind _gunowner (`self.GunOwner`))
  (bind _returnvalue (`SceneComponent.K2_GetComponentLocation` (`/Game/Blueprints/FppCore/FppShooter.Camera` _gunowner)))
  (bind (_outhit _returnvalue_2) (`KismetSystemLibrary.LineTraceSingle` :`Start` _returnvalue :`End` (+ _returnvalue (* (`KismetMathLibrary.Normal` (`KismetMathLibrary.GetForwardVector` (`Pawn.GetControlRotation` _gunowner))) 1500)) :`TraceChannel` "TraceTypeQuery1" :`DrawDebugType` "ForDuration"))
  (if _returnvalue_2
    (bind _asrobot_shooter (cast `/Game/Blueprints/TppCore/RobotShooter` (`.HitActor` (`GameplayStatics.BreakHitResult` _outhit))))
    (`/Game/Blueprints/TppCore/RobotShooter.TakeDamage` _asrobot_shooter 20.0)))

(fn `UserConstructionScript`
  (`parent.UserConstructionScript`))