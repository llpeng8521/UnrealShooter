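; Launcher weapon Blueprint that fires PhysicsBullet projectiles for its owning character.
; StartFire triggers a single shot through ShootOnce, and EndFire does nothing, so there is no automatic fire.
; ShootOnce rate-limits shots by the fire animation length, spawns the bullet at the Muzzle using the owner's control rotation, then plays the first-person launcher fire montage on the owner.
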(event `self.StartFire`
  (`self.ShootOnce`))

(event `self.EndFire`)

(event `self.ShootOnce`
  (if (>= (- (`GameplayStatics.GetTimeSeconds`) (`self.LastShootTime`)) (`self.ShootAnimTimeLength`))
    (set `self.LastShootTime` (`GameplayStatics.GetTimeSeconds`))
    (`|SpawnActorFromClass` "/Game/Blueprints/PhysicsBullet.PhysicsBullet_C" (`KismetMathLibrary.MakeTransform` (`SceneComponent.K2_GetComponentLocation` (`self.Muzzle`)) (`Pawn.GetControlRotation` (`self.GunOwner`))) "Undefined" "OverrideRootScale" null null)
    (`Character.PlayAnimMontage` (`self.GunOwner`) "/Game/Blueprints/FppCore/FppLauncherFire_Montage.FppLauncherFire_Montage" 1.0 "None")))

(fn `UserConstructionScript`
  (`parent.UserConstructionScript`))