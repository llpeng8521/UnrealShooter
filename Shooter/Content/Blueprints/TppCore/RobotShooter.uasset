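; RobotShooter is a robot pawn that tracks health, takes damage and removes itself from the game on death.
; Its construction script sets the mesh to block the Visibility channel, so traces on that channel can hit it.
; TakeDamage subtracts from Health and prints it; at zero or below, it detaches the controller and starts a short timer to OnDieOver, which destroys the actor.
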(fn `IsDead`
  (returns (bDead :type Boolean))
  (return (<= (`self.Health`) 0.0)))

(fn `OnDieOver`
  (`self.K2_DestroyActor`))

(fn `TakeDamage`
  (params (Damage :type "Float (double-precision)"))
  (bind _output_get (set `self.Health` (- (`self.Health`) Damage)))
  (`KismetSystemLibrary.PrintString` (`KismetStringLibrary.Conv_DoubleToString` _output_get))
  (if (`self.IsDead`)
    (`self.DetachFromControllerPendingDestroy`)
    (`KismetSystemLibrary.K2_SetTimer` null "OnDieOver" 1.2)))

(fn `UserConstructionScript`
  (`PrimitiveComponent.SetCollisionResponseToChannel` (`self.Mesh`) "ECC_Visibility" "ECR_Block"))